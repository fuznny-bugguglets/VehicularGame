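; BP_MainMenuAudio is a Blueprint that plays occasional radio interception audio for the main menu.
; RadioInterceptions starts on BeginPlay and re-calls itself after delays, forming an endless timed loop with a one-in-five chance to play on each pass.
; A successful roll primes the MainMenuAudio cue, adds a new audio component and waits an extra cooldown before looping.
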(event Custom|RadioInterceptions
  ;[0.2956 0.3941 1] Determine if sound plays
  (Utilities|FlowControl|Delay 15.0)
  (if (< (Math|Random|RandomIntegerinRange 0 4) 1)
    ;[1 0.4842 0.857] Play sound + reset
    (Class|AudioMixerBlueprintLibrary|PrimeSoundCueforPlayback "/Game/Sounds/MainMenu/MainMenuAudio.MainMenuAudio")
    (AddComponent|AddAudioComponent false)
    (Utilities|FlowControl|Delay 1e+01)
    (CallFunction|RadioInterceptions)
    (else
      (CallFunction|RadioInterceptions))))

(event EventBeginPlay
  ;[0.1546 1 0] Start the whole thing
  (CallFunction|RadioInterceptions))

(fn ConstructionScript)