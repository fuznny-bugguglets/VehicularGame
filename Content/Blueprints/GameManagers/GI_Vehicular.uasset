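; GI_Vehicular is a game instance holding two deprecated upgrade helper functions, apparently kept to expose any remaining callers.
; CanPlayerAfford prints a debug warning and always returns false, leaving its banked scrap, components and relics check unused.
; IsUpgradeUnlocked prints a similar warning and always returns true.
; Its old check of prerequisite upgrade IDs against purchases in BP_VehicularSaveGame remains as unreachable logic.
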(fn CanPlayerAfford
  (params (CommonCost :type Integer) (UncommonCost :type Integer) (RareCost :type Integer))
  (Development|PrintString "tell charlie that old can player afford code in game instance is running")
  (return false))

(fn IsUpgradeUnlocked
  (params (PrerequisiteUpgradeIDs :type Array%20of%20Names))
  (Development|PrintString "let charlie know that old upgrade unlocked code is running")
  (return true))