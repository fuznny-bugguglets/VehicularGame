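; Monster closet area that spawns waves of enemies at a SPAWN point while a BP_Vehicle overlaps it.
; Entering sets POIStarted and, after a short delay, starts a small-enemy loop, then a medium-enemy loop a minute later.
; Each loop repeats through its own Delay while the flag holds.
; Exit clears the flag, but a pending delay still yields one more spawn because the check precedes the wait.
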(event Custom|MediumEnemy
  (if (Variables|Default|GetPOIStarted)
    (Game|SpawnActorfromClass "/Game/Blueprints/Enemies/Classes/MediumEnemy.MediumEnemy_C" (Math|Conversions|ToTransform(Vector) (Transformation|GetWorldLocation (Variables|/Script/Engine.Actor|GetRootComponent (Variables|Default|GetSPAWN)))) "Undefined" "MultiplyWithRoot" 0 0 :!label _label)
    (if (Variables|Default|GetPOIStarted)
      (Utilities|FlowControl|Delay 25.0)
      (goto _label))))

(event Custom|SmallEnemy
  (if (Variables|Default|GetPOIStarted)
    (Game|SpawnActorfromClass "/Game/Blueprints/Enemies/Classes/SmallEnemy.SmallEnemy_C" (Math|Conversions|ToTransform(Vector) (Transformation|GetWorldLocation (Variables|/Script/Engine.Actor|GetRootComponent (Variables|Default|GetSPAWN)))) "Undefined" "MultiplyWithRoot" 0 0 :!label _label)
    (if (Variables|Default|GetPOIStarted)
      (Utilities|FlowControl|Delay 2e+01)
      (goto _label))))

(event Collision|EventActorBeginOverlap
  (params (OtherActor :type Actor%20Object%20Reference))
  ;[1 1 1] Sets POIStarted to True on vehicle overlap
  (Utilities|Casting|CastToBP_Vehicle OtherActor)
  (Variables|Default|SetPOIStarted true)
  (Utilities|FlowControl|Delay 5.0)
  (if true
    (CallFunction|SmallEnemy)
    (Utilities|FlowControl|Delay 6e+01)
    (CallFunction|MediumEnemy)))

(event Collision|EventActorEndOverlap
  (params (OtherActor :type Actor%20Object%20Reference))
  (Utilities|Casting|CastToBP_Vehicle OtherActor)
  (Variables|Default|SetPOIStarted false))

(fn ConstructionScript)