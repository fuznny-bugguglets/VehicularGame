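; BP_Ruin is a resource ruin with an extraction ring, holding a depletable amount of Mechanical, Electronic or Robotic resource.
; The construction script uses the resource type to pick the ring material and show only the matching common, uncommon or rare mesh.
; One tick after BeginPlay, it restores its amount from GI_Vehicular's save data, keyed by display name, or defaults to the maximum.
; UpdateBubble clears the ring mesh when the resource is depleted.
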(event Custom|UpdateBubble
  (if (<= (Variables|Default|GetResourceAmount) 0)
    (Components|StaticMesh|SetStaticMesh (Variables|Default|GetExtractionRingVisual) 0)))

(event EventBeginPlay
  (Utilities|FlowControl|DelayUntilNextTick)
  (bind _asgi_vehicular (Utilities|Casting|CastToGI_Vehicular (Game|GetGameInstance)))
  (if (.ReturnValue (Utilities|Map|Find (Variables|/Script/VehicularGame.VehicularSaveGame|GetRuinResourceData (Variables|/Script/VehicularGame.VehicularGameInstance|GetSaveGameObject _asgi_vehicular)) (Utilities|String|StringToName (Utilities|GetDisplayName self))))
    (Variables|Default|SetResourceAmount (.Value (Utilities|Map|Find (Variables|/Script/VehicularGame.VehicularSaveGame|GetRuinResourceData (Variables|/Script/VehicularGame.VehicularGameInstance|GetSaveGameObject _asgi_vehicular)) (Utilities|String|StringToName (Utilities|GetDisplayName self)))))
    (CallFunction|UpdateBubble)
    (else
      (Variables|Default|SetResourceAmount (Variables|Default|GetMaxResourceAmount)))))

(event Collision|EventActorBeginOverlap
  (params (OtherActor :type Actor%20Object%20Reference)))

(event EventTick
  (params (DeltaSeconds :type Float%20%28single-precision%29)))

(fn ConstructionScript
  (bind _ruinmeshcommon (Variables|Default|GetRuinMeshCommon))
  (bind _resourcetype (Variables|Default|GetResourceType))
  (bind _ruinmeshuncommon (Variables|Default|GetRuinMeshUncommon))
  (bind _ruinmeshrare (Variables|Default|GetRuinMeshRare))
  (Rendering|Material|SetMaterial (Variables|Default|GetExtractionRingVisual) 0 (Utilities|Select :Index _resourcetype :NewEnumerator0 (Variables|Default|GetRadiusScrapMaterial) :NewEnumerator1 (Variables|Default|GetRadiusComponentMaterial) :NewEnumerator2 (Variables|Default|GetRadiusRelicMaterial)))
  (switch Utilities|FlowControl|Switch|SwitchonResourceType _resourcetype
    (:NewEnumerator0
      (Utilities|FlowControl|Sequence
        (:then_0
          (Rendering|SetVisibility _ruinmeshrare false false :!label _label)
          (Collision|SetCollisionEnabled _ruinmeshrare "NoCollision"))
        (:then_1
          (Rendering|SetVisibility _ruinmeshuncommon false false :!label _label_2)
          (Collision|SetCollisionEnabled _ruinmeshuncommon "NoCollision"))))
    (:NewEnumerator1
      (Utilities|FlowControl|Sequence
        (:then_0
          (goto _label))
        (:then_1
          (Rendering|SetVisibility _ruinmeshcommon false false :!label _label_3)
          (Collision|SetCollisionEnabled _ruinmeshcommon "NoCollision"))))
    (:NewEnumerator2
      (Utilities|FlowControl|Sequence
        (:then_0
          (goto _label_2))
        (:then_1
          (goto _label_3))))))