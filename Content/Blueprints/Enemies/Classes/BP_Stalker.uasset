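; BP_Stalker is an enemy actor that travels along the spline of a referenced actor, starting on BeginPlay.
; A timeline, with play rate set to the inverse of TimeToComplete, maps its track value to a distance along the spline's length.
; Each update sets the world location at that distance, while rotation is always sampled at the spline's start, so it does not follow the curve.
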(event EventBeginPlay
  (bind _splinereference (Variables|Default|GetSplineReference))
  (bind _spline (Variables|/Game/Blueprints/BP_Spline.BP_Spline_C|GetSpline _splinereference))
  (Components|Timeline|SetPlayRate (Variables|Default|GetT_Move) (/ 1.0 (Variables|Default|GetTimeToComplete)))
  (bind _movetrack (Timeline|T_Move Play)
    (:Update
      (Transformation|SetActorLocationAndRotation (Spline|GetLocationatDistanceAlongSpline _spline (Math|Float|Lerp 0.0 (Spline|GetSplineLength _spline) _movetrack) "World") (Spline|GetRotationatDistanceAlongSpline _spline 0.0 "World")))))

(fn ConstructionScript)