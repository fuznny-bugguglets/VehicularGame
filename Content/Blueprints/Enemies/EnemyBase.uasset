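; Base enemy character that chases the player's vehicle, damages it on contact and gets knocked away by it.
; Tick scales walk speed from player speed through a curve with rate-limited smoothing, and tilts the mesh to ground slope.
; Timed navigation updates target a blend of player position and the AI controller's moving target, weighted by player speed.
; Overlap damages a slow player or one not hitting head-on, then launches the enemy away.
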(event Custom|DamagePlayer
  (Game|Damage|ApplyDamage (Game|Player|GetPlayerPawn 0) 5.0 0 0))

(event Custom|PathfindToPoint
  (params (DeltaTime :type Float%20%28double-precision%29))
  (bind _returnvalue (Game|Player|GetPlayerPawn 0))
  (bind _self self)
  (bind _returnvalue_2 (Transformation|GetActorTransform _returnvalue))
  (bind (_projectedlocation _returnvalue_3) (AI|Navigation|ProjectPointtoNavigation (.location _returnvalue_2) 0 0 "350.000000,350.000000,350.000000"))
  (bind _output_get (Variables|Default|SetTimeSinceLastNavUpdate (+ (Variables|Default|GetTimeSinceLastNavUpdate) DeltaTime)))
  (if (> _output_get (Variables|Default|GetTimeBetweenNavUpdates))
    (Variables|Default|SetTimeSinceLastNavUpdate 0.0)
    (if (not (Class|EnemyCharacter|IsDead))
      (bind _asbp_enemy_aicontroller (Utilities|Casting|CastToBP_EnemyAIController (AI|GetAIController _self)))
      (Utilities|IsValid _returnvalue
        (:Is%20Valid
          (if (.ReturnValue (AI|Navigation|ProjectPointtoNavigation (Utilities|VectorInterpEaseinOut (.location _returnvalue_2) (Class|EnemyAIController|GetMovingTargetLocation _asbp_enemy_aicontroller) (Math|Float|Clamp(Float) (/ (Variables|Default|GetPlayerSpeed) (* (Variables|Default|GetPlayerMinSpeed) 27.77))) 5.0) 0 0 "350.000000,350.000000,350.000000"))
            (AI|AIMoveTo _self (.ProjectedLocation (AI|Navigation|ProjectPointtoNavigation (Utilities|VectorInterpEaseinOut (.location _returnvalue_2) (Class|EnemyAIController|GetMovingTargetLocation _asbp_enemy_aicontroller) (Math|Float|Clamp(Float) (/ (Variables|Default|GetPlayerSpeed) (* (Variables|Default|GetPlayerMinSpeed) 27.77))) 5.0) 0 0 "350.000000,350.000000,350.000000")) 0 1.0 false)
            (else
              (AI|AIMoveTo _self (Math|Vector|SelectVector _projectedlocation (.location _returnvalue_2) _returnvalue_3) 0 1.0 false))))))))

(event Custom|UpdateSpeed
  (params (Delta%20Seconds :type Float%20%28double-precision%29))
  (bind _returnvalue (Game|Player|GetPlayerPawn 0))
  (bind _self self)
  (bind _charactermovement (Variables|Character|GetCharacterMovement))
  (bind _returnvalue_2 (Transformation|GetActorTransform _returnvalue))
  (bind _output_get (Variables|Default|SetPlayerSpeed (/ (Math|Vector|Distance(Vector) (.location _returnvalue_2) (Variables|Default|GetLastPlayerPosition)) Delta%20Seconds)))
  (Variables|Default|SetLastPlayerPosition (.location _returnvalue_2))
  (bind _output_get_2 (Variables|Default|SetSpeedScalingCurve (Variables|Default|GetSpeedScalingCurve)))
  (bind _asenemy_aicontroller (Utilities|Casting|CastToEnemyAIController (AI|GetAIController _self)))
  (bind _output_get_3 (Variables|Default|SetTargetSpeed (Math|Float|SelectFloat (- (Variables|Default|GetTargetSpeed) (* Delta%20Seconds (Variables|Default|GetCloseToPlayerDecelleration))) (+ (Math|Curves|GetFloatValue _output_get_2 (* _output_get 0.01 3.666)) (* _output_get 0.01 3.666)) (< (Math|Vector|Distance(Vector) (.location (Transformation|GetActorTransform _self)) (Class|EnemyAIController|GetMovingTargetLocation _asenemy_aicontroller)) (Variables|/Script/VehicularGame.EnemyAIController|GetTargetLineForwardOffset _asenemy_aicontroller)))))
  (if (> (Variables|Default|GetRollingAverageTargetSpeed) _output_get_3)
    (bind _output_get_4 (Variables|Default|SetRollingAverageTargetSpeed (+ (* (Variables|Default|GetSpeedChangeRatePerSec) Delta%20Seconds) (Variables|Default|GetRollingAverageTargetSpeed))))
    (Variables|/Script/Engine.CharacterMovementComponent|SetMaxWalkSpeed _charactermovement (* (Math|Float|Clamp(Float) _output_get_4 (Variables|Default|GetRollingAverageTargetSpeed) (Variables|Default|GetTargetSpeed)) 1e+02 0.272777))
    (else
      (bind _output_get_5 (Variables|Default|SetRollingAverageTargetSpeed (+ (Variables|Default|GetRollingAverageTargetSpeed) (* (Variables|Default|GetSpeedChangeRatePerSec) (* Delta%20Seconds -1.0)))))
      (Variables|/Script/Engine.CharacterMovementComponent|SetMaxWalkSpeed _charactermovement (* (Math|Float|Clamp(Float) _output_get_5 (Variables|Default|GetTargetSpeed) (Variables|Default|GetRollingAverageTargetSpeed)) 1e+02 0.272777)))))

(event Custom|HitByPlayer
  (bind _returnvalue (Transformation|GetActorLocation))
  (bind _returnvalue_2 (Game|Player|GetPlayerPawn 0))
  (bind _playerpushforce (Variables|Default|GetPlayerPushForce))
  (bind _returnvalue_3 (Transformation|GetActorLocation _returnvalue_2))
  (bind _returnvalue_4 (Math|Vector|GetUnitDirection(Vector) _returnvalue_3 _returnvalue))
  (bind _returnvalue_5 (Math|Vector|MakeVector (.x _returnvalue_4) (.y _returnvalue_4) 0.1))
  (bind _returnvalue_6 (* _returnvalue_5 _playerpushforce))
  (bind _asstatic_mesh_component (Utilities|Casting|CastToStaticMeshComponent (Variables|/Script/Engine.Actor|GetRootComponent _returnvalue_2)))
  (bind _returnvalue_7 (Physics|GetPhysicsLinearVelocity _asstatic_mesh_component "None"))
  (Pawn|Components|CharacterMovement|SetMovementMode (Variables|Character|GetCharacterMovement) "MOVE_Falling" 0)
  (Character|LaunchCharacter (select (> (.x (Math|Transform|InverseTransformLocation (Transformation|GetActorTransform _returnvalue_2) (Transformation|GetActorLocation))) 2.5e+02) (+ _returnvalue_7 _returnvalue_6) _returnvalue_6) false false))

(event Custom|RotateToGround
  (params (Delta%20Seconds :type Float%20%28double-precision%29))
  (bind _self self)
  (bind _cube (Variables|Default|GetCube))
  (bind _returnvalue (Transformation|GetWorldRotation _cube))
  (bind _rootcomponent (Variables|/Script/Engine.Actor|GetRootComponent _self))
  (bind _returnvalue_2 (Transformation|GetWorldLocation _rootcomponent))
  (bind _outhit (Collision|LineTraceByChannel _returnvalue_2 (- _returnvalue_2 (* (Math|Vector|GetUpVector (Variables|/Script/Engine.Actor|GetRootComponent _self)) 1e+03)) "TraceTypeQuery1" false 0 "None"))
  (Transformation|SetWorldRotation (Variables|Default|GetCube) (Math|Interpolation|RInterpTo _returnvalue (Math|Rotator|MakeRotator (* (.OutSlopeRollDegreeAngle (Class|KismetMathLibrary|GetSlopeDegreeAngles (Transformation|GetActorRightVector) (.impactnormal _outhit) (Transformation|GetActorUpVector))) -1.0) (.OutSlopePitchDegreeAngle (Class|KismetMathLibrary|GetSlopeDegreeAngles (Transformation|GetActorRightVector) (.impactnormal _outhit) (Transformation|GetActorUpVector))) (.Yaw (Math|Rotator|BreakRotator _returnvalue))) Delta%20Seconds 2.0) false false))

(event Collision|EventActorEndOverlap
  (params (OtherActor :type Actor%20Object%20Reference))
  (if (== OtherActor (Game|Player|GetPlayerPawn 0))
    (Variables|Default|SetisOverlappingWithPlayer false)))

(event Collision|EventActorBeginOverlap
  (params (OtherActor :type Actor%20Object%20Reference))
  (bind _returnvalue (Game|Player|GetPlayerPawn 0))
  (if (== OtherActor _returnvalue)
    (Variables|Default|SetisOverlappingWithPlayer true)
    (if (or (< (Variables|Default|GetPlayerSpeed) 15.0) (< (.x (Math|Transform|InverseTransformLocation (Transformation|GetActorTransform _returnvalue) (Transformation|GetActorLocation))) 2e+02))
      (Audio|PlaySoundatLocation "/Game/Sounds/Vehicle/Hit_by_enemy_just_thump.Hit_by_enemy_just_thump" "0, 0, 0" "0, 0, 0" 1.0 1.0 0.0 0 0 0 0)
      (CallFunction|DamagePlayer))))

(event EventTick
  (params (DeltaSeconds :type Float%20%28single-precision%29))
  (CallFunction|UpdateSpeed DeltaSeconds)
  (CallFunction|RotatetoGround DeltaSeconds)
  (CallFunction|PathfindtoPoint DeltaSeconds)
  (if (Variables|Default|GetisOverlappingWithPlayer)
    (CallFunction|HitbyPlayer)))

(fn ConstructionScript)