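; BigEnemy is an enemy character whose max walk speed is driven by the player's movement speed.
; Each Tick derives player speed from position change, converts it to approximate km/h and adds a SpeedScalingCurve offset to get a target.
; A rolling speed steps up by SpeedChangeRatePerSec when above that target, otherwise down.
; Its value, clamped against the target and converted back to cm/s, sets MaxWalkSpeed.
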(event EventBeginPlay)

(event Collision|EventActorBeginOverlap
  (params (OtherActor :type Actor%20Object%20Reference)))

(event EventTick
  (params (DeltaSeconds :type Float%20%28single-precision%29))
  (bind _returnvalue (Game|Player|GetPlayerPawn 0))
  (bind _charactermovement (Variables|Character|GetCharacterMovement))
  (bind _returnvalue_2 (Transformation|GetActorTransform _returnvalue))
  (bind _output_get (Variables|Default|SetPlayerSpeed (/ (Math|Vector|Distance(Vector) (.location _returnvalue_2) (Variables|Default|GetLastPlayerPosition)) DeltaSeconds)))
  (Variables|Default|SetLastPlayerPosition (.location _returnvalue_2))
  (bind _output_get_2 (Variables|Default|SetSpeedScalingCurve (Variables|Default|GetSpeedScalingCurve)))
  (bind _output_get_3 (Variables|Default|SetTargetSpeed (+ (Math|Curves|GetFloatValue _output_get_2 (* _output_get 0.01 3.666)) (* _output_get 0.01 3.666))))
  (if (> (Variables|Default|GetRollingAverageTargetSpeed) _output_get_3)
    (bind _output_get_4 (Variables|Default|SetRollingAverageTargetSpeed (+ (* (Variables|Default|GetSpeedChangeRatePerSec) DeltaSeconds) (Variables|Default|GetRollingAverageTargetSpeed))))
    (Variables|/Script/Engine.CharacterMovementComponent|SetMaxWalkSpeed _charactermovement (* (Math|Float|Clamp(Float) _output_get_4 (Variables|Default|GetRollingAverageTargetSpeed) (Variables|Default|GetTargetSpeed)) 1e+02 0.272777))
    (else
      (bind _output_get_5 (Variables|Default|SetRollingAverageTargetSpeed (+ (Variables|Default|GetRollingAverageTargetSpeed) (* (Variables|Default|GetSpeedChangeRatePerSec) (* DeltaSeconds -1.0)))))
      (Variables|/Script/Engine.CharacterMovementComponent|SetMaxWalkSpeed _charactermovement (* (Math|Float|Clamp(Float) _output_get_5 (Variables|Default|GetTargetSpeed) (Variables|Default|GetRollingAverageTargetSpeed)) 1e+02 0.272777)))))

(fn ConstructionScript)