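; Vehicle-mounted gatling turret that aims with the vehicle camera and fires bullets while fire is held.
; On init it receives the camera and shooter pawn, then each Tick the TurretRotator interpolates the head toward the camera transform.
; A timer gated by Firerate limits shots, which alternate between left and right spawn points, each with its own gunshot sound and the shooter as instigator.
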(event EventBeginPlay)

(event Collision|EventActorBeginOverlap
  (params (OtherActor :type Actor%20Object%20Reference)))

(event EventTick
  (params (DeltaSeconds :type Float%20%28single-precision%29))
  (Class|TurretRotationComponent|RotateTurretHead (Variables|Default|GetTurretRotator) (Transformation|GetWorldTransform (Variables|Default|GetVehicleCamera)) DeltaSeconds 1e+04 2e+01)
  (if (< (Variables|Default|GetTimeSinceLastShot) (/ 1.0 (Variables|Default|GetFirerate)))
    (Variables|Default|SetTimeSinceLastShot (+ (Variables|Default|GetTimeSinceLastShot) DeltaSeconds))))

(event EventFireReleased)

(event EventFireheld
  (if (> (Variables|Default|GetTimeSinceLastShot) (/ 1.0 (Variables|Default|GetFirerate)))
    (if (Variables|Default|GetLeftShotLast)
      (Variables|Default|SetLeftShotLast false)
      (Game|SpawnActorfromClass "/Game/Blueprints/Bullet.Bullet_C" (Transformation|GetWorldTransform (Variables|Default|GetBulletSpawnR)) "Undefined" "MultiplyWithRoot" 0 (Variables|Default|GetShooterPawn))
      (Audio|PlaySound2D "/Game/Sounds/Vehicle/Gunshot_Pitch_2.Gunshot_Pitch_2" 1.0 1.0 0.0 0 0)
      (else
        (Variables|Default|SetLeftShotLast true)
        (Game|SpawnActorfromClass "/Game/Blueprints/Bullet.Bullet_C" (Transformation|GetWorldTransform (Variables|Default|GetBulletSpawnL)) "Undefined" "MultiplyWithRoot" 0 (Variables|Default|GetShooterPawn))
        (Audio|PlaySound2D "/Game/Sounds/Vehicle/Gunshot_Pitch_1.Gunshot_Pitch_1" 1.0 1.0 0.0 0 0)))
    (Variables|Default|SetTimeSinceLastShot 0.0)))

(event EventFirePressed)

(event EventTurretInitializeVariables
  (params (CameraComponent :type Camera%20Component%20Object%20Reference%20%28by%20ref%29) (ShootingPawn :type Pawn%20Object%20Reference))
  (Variables|Default|SetVehicleCamera CameraComponent)
  (Variables|Default|SetShooterPawn ShootingPawn))

(fn ConstructionScript)