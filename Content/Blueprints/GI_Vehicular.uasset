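; Game instance for a vehicle scavenging game that handles the end of a successful run.
; On run success it banks the player vehicle's scrap, components and relics into the save object and zeroes the carried counts.
; It also rebuilds a name-keyed map of each ruin actor's remaining resources, then saves and opens the upgrade level.
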(event Custom|Bank%20Inventory
  (bind _savegameobject (Variables|Default|GetSaveGameObject))
  (Utilities|IsValid _savegameobject
    (:Is%20Valid
      (bind _asvehicle (Utilities|Casting|CastToVehicle (Game|Player|GetPlayerPawn 0)))
      (Utilities|IsValid _asvehicle
        (:Is%20Valid
          (Variables|/Script/VehicularGame.VehicularSaveGame|SetBankedScrap _savegameobject (+ (Variables|/Game/Blueprints/Vehicle.Vehicle_C|GetScrapCount _asvehicle) (Variables|/Script/VehicularGame.VehicularSaveGame|GetBankedScrap _savegameobject)))
          (Variables|/Script/VehicularGame.VehicularSaveGame|SetBankedComponents _savegameobject (+ (Variables|/Game/Blueprints/Vehicle.Vehicle_C|GetComponentCount _asvehicle) (Variables|/Script/VehicularGame.VehicularSaveGame|GetBankedComponents _savegameobject)))
          (Variables|/Script/VehicularGame.VehicularSaveGame|SetBankedRelics _savegameobject (+ (Variables|/Game/Blueprints/Vehicle.Vehicle_C|GetRelicCount _asvehicle) (Variables|/Script/VehicularGame.VehicularSaveGame|GetBankedRelics _savegameobject)))
          (Variables|/Game/Blueprints/Vehicle.Vehicle_C|SetScrapCount _asvehicle 0)
          (Variables|/Game/Blueprints/Vehicle.Vehicle_C|SetComponentCount _asvehicle 0)
          (Variables|/Game/Blueprints/Vehicle.Vehicle_C|SetRelicCount _asvehicle 0))))))

(event Custom|Save%20Ruin%20resources
  (Utilities|Map|Clear (Variables|/Script/VehicularGame.VehicularSaveGame|GetRuinResourceData (Variables|Default|GetSaveGameObject)))
  (bind _outactors (Actor|GetAllActorsOfClass "/Game/Blueprints/BP_Ruin.BP_Ruin_C"))
  (for _array_element _outactors
    (Utilities|Map|Add (Variables|/Script/VehicularGame.VehicularSaveGame|GetRuinResourceData (Variables|Default|GetSaveGameObject)) (Utilities|String|StringToName (Utilities|GetDisplayName _array_element)) (Variables|/Game/Blueprints/BP_Ruin.BP_Ruin_C|GetResourceAmount _array_element))))

(event EventOnRunSuccess
  (CallFunction|BankInventory)
  (CallFunction|SaveRuinResources)
  (Class|VehicularGameInstance|SaveGameData)
  (Game|OpenLevel(byName) "UpgradeLevel"))