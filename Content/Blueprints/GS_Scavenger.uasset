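; Scavenger game state that turns the player's purchased upgrades into stat values for the vehicular game.
; On BeginPlay it gets the save object from GI_Vehicular and reads its UpgradePurchasedStatus map.
; A chain of events sets health, speed, boost, damage, projectile, fire rate and bumper values in turn.
; Upgrade tiers are nested checks, so a higher tier counts only if the lower ones are purchased.
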(event Custom|SetAdditionalMaxHealth
  (if (.Value (Utilities|Map|Find (Variables|/Game/Blueprints/BP_VehicularSaveGame.BP_VehicularSaveGame_C|GetUpgradePurchasedStatus (Variables|Default|GetBPVehicularSaveGame)) "HealthUpgrade1"))
    (Variables|Default|SetAdditionalMaxHealth (+ (Variables|Default|GetAdditionalMaxHealth) 25.0))
    (if (.Value (Utilities|Map|Find (Variables|/Game/Blueprints/BP_VehicularSaveGame.BP_VehicularSaveGame_C|GetUpgradePurchasedStatus (Variables|Default|GetBPVehicularSaveGame)) "HealthUpgrade2"))
      (Variables|Default|SetAdditionalMaxHealth (+ (Variables|Default|GetAdditionalMaxHealth) 25.0))
      (if (.Value (Utilities|Map|Find (Variables|/Game/Blueprints/BP_VehicularSaveGame.BP_VehicularSaveGame_C|GetUpgradePurchasedStatus (Variables|Default|GetBPVehicularSaveGame)) "HealthUpgrade3"))
        (Variables|Default|SetAdditionalMaxHealth (+ (Variables|Default|GetAdditionalMaxHealth) 25.0))
        (if (.Value (Utilities|Map|Find (Variables|/Game/Blueprints/BP_VehicularSaveGame.BP_VehicularSaveGame_C|GetUpgradePurchasedStatus (Variables|Default|GetBPVehicularSaveGame)) "HealthUpgrade4"))
          (Variables|Default|SetAdditionalMaxHealth (+ (Variables|Default|GetAdditionalMaxHealth) 25.0)))
        (CallFunction|SetAdditionalMaxSpeed)
        (else
          (CallFunction|SetAdditionalMaxSpeed)))
      (else
        (CallFunction|SetAdditionalMaxSpeed)))
    (else
      (CallFunction|SetAdditionalMaxSpeed))))

(event Custom|SetProjectileSpeedAndSpreadMultiplier
  (if (.Value (Utilities|Map|Find (Variables|/Game/Blueprints/BP_VehicularSaveGame.BP_VehicularSaveGame_C|GetUpgradePurchasedStatus (Variables|Default|GetBPVehicularSaveGame)) "BulletSpeedUpgrade1"))
    (Variables|Default|SetProjectileSpeedMultiplier 2.0)
    (Variables|Default|SetProjectileSpreadMultiplier 0.4)
    (if (.Value (Utilities|Map|Find (Variables|/Game/Blueprints/BP_VehicularSaveGame.BP_VehicularSaveGame_C|GetUpgradePurchasedStatus (Variables|Default|GetBPVehicularSaveGame)) "BulletSpeedUpgrade2"))
      (Variables|Default|SetProjectileSpeedMultiplier 4.0)
      (Variables|Default|SetProjectileSpreadMultiplier 0.1))
    (CallFunction|SetFireRateUpgradeLevel)
    (else
      (CallFunction|SetFireRateUpgradeLevel))))

(event Custom|SetBumperDamage
  (if (.Value (Utilities|Map|Find (Variables|/Game/Blueprints/BP_VehicularSaveGame.BP_VehicularSaveGame_C|GetUpgradePurchasedStatus (Variables|Default|GetBPVehicularSaveGame)) "BumperDamageUpgrade1"))
    (Variables|Default|SetBumperDamage 1e+01)
    (if (.Value (Utilities|Map|Find (Variables|/Game/Blueprints/BP_VehicularSaveGame.BP_VehicularSaveGame_C|GetUpgradePurchasedStatus (Variables|Default|GetBPVehicularSaveGame)) "BumperDamageUpgrade2"))
      (Variables|Default|SetBumperDamage 2e+01)
      (if (.Value (Utilities|Map|Find (Variables|/Game/Blueprints/BP_VehicularSaveGame.BP_VehicularSaveGame_C|GetUpgradePurchasedStatus (Variables|Default|GetBPVehicularSaveGame)) "BumperDamageUpgrade3"))
        (Variables|Default|SetBumperDamage 3e+01)))))

(event Custom|SetFireRateUpgradeLevel
  (if (.Value (Utilities|Map|Find (Variables|/Game/Blueprints/BP_VehicularSaveGame.BP_VehicularSaveGame_C|GetUpgradePurchasedStatus (Variables|Default|GetBPVehicularSaveGame)) "FireRateUpgrade1"))
    (Variables|Default|SetFireRateUpgradeLevel 1)
    (if (.Value (Utilities|Map|Find (Variables|/Game/Blueprints/BP_VehicularSaveGame.BP_VehicularSaveGame_C|GetUpgradePurchasedStatus (Variables|Default|GetBPVehicularSaveGame)) "FireRateUpgrade2"))
      (Variables|Default|SetFireRateUpgradeLevel 2)
      (if (.Value (Utilities|Map|Find (Variables|/Game/Blueprints/BP_VehicularSaveGame.BP_VehicularSaveGame_C|GetUpgradePurchasedStatus (Variables|Default|GetBPVehicularSaveGame)) "FireRateUpgrade3"))
        (Variables|Default|SetFireRateUpgradeLevel 3))
      (CallFunction|SetProjectilePiercing)
      (else
        (CallFunction|SetProjectilePiercing)))
    (else
      (CallFunction|SetProjectilePiercing))))

(event Custom|SetProjectilePiercing
  (if (.Value (Utilities|Map|Find (Variables|/Game/Blueprints/BP_VehicularSaveGame.BP_VehicularSaveGame_C|GetUpgradePurchasedStatus (Variables|Default|GetBPVehicularSaveGame)) "ProjectilePiercingUpgrade1"))
    (Variables|Default|SetProjectilePiercing 1)
    (if (.Value (Utilities|Map|Find (Variables|/Game/Blueprints/BP_VehicularSaveGame.BP_VehicularSaveGame_C|GetUpgradePurchasedStatus (Variables|Default|GetBPVehicularSaveGame)) "ProjectilePiercingUpgrade2"))
      (Variables|Default|SetProjectilePiercing 2))
    (CallFunction|SetBumperDamage)
    (else
      (CallFunction|SetBumperDamage))))

(event Custom|SetMaxBoostLevel
  (if (.Value (Utilities|Map|Find (Variables|/Game/Blueprints/BP_VehicularSaveGame.BP_VehicularSaveGame_C|GetUpgradePurchasedStatus (Variables|Default|GetBPVehicularSaveGame)) "BoostUpgrade1"))
    (Variables|Default|SetmaxBoostLevel (+ (Variables|Default|GetmaxBoostLevel) 1))
    (if (.Value (Utilities|Map|Find (Variables|/Game/Blueprints/BP_VehicularSaveGame.BP_VehicularSaveGame_C|GetUpgradePurchasedStatus (Variables|Default|GetBPVehicularSaveGame)) "BoostUpgrade2"))
      (Variables|Default|SetmaxBoostLevel (+ (Variables|Default|GetmaxBoostLevel) 1)))
    (CallFunction|SetAdditionalDamage)
    (else
      (CallFunction|SetAdditionalDamage))))

(event Custom|SetAdditionalMaxSpeed
  (if (.Value (Utilities|Map|Find (Variables|/Game/Blueprints/BP_VehicularSaveGame.BP_VehicularSaveGame_C|GetUpgradePurchasedStatus (Variables|Default|GetBPVehicularSaveGame)) "SpeedUpgrade1"))
    (Variables|Default|SetAdditionalMaxSpeed (+ (Variables|Default|GetAdditionalMaxSpeed) 1e+01))
    (if (.Value (Utilities|Map|Find (Variables|/Game/Blueprints/BP_VehicularSaveGame.BP_VehicularSaveGame_C|GetUpgradePurchasedStatus (Variables|Default|GetBPVehicularSaveGame)) "SpeedUpgrade2"))
      (Variables|Default|SetAdditionalMaxSpeed (+ (Variables|Default|GetAdditionalMaxSpeed) 1e+01)))
    (CallFunction|SetMaxBoostLevel)
    (else
      (CallFunction|SetMaxBoostLevel))))

(event Custom|SetAdditionalDamage
  (if (.Value (Utilities|Map|Find (Variables|/Game/Blueprints/BP_VehicularSaveGame.BP_VehicularSaveGame_C|GetUpgradePurchasedStatus (Variables|Default|GetBPVehicularSaveGame)) "DamageUpgrade1"))
    (Variables|Default|SetAdditionalDamage (+ (Variables|Default|GetAdditionalDamage) 5.0))
    (if (.Value (Utilities|Map|Find (Variables|/Game/Blueprints/BP_VehicularSaveGame.BP_VehicularSaveGame_C|GetUpgradePurchasedStatus (Variables|Default|GetBPVehicularSaveGame)) "DamageUpgrade2"))
      (Variables|Default|SetAdditionalDamage (+ (Variables|Default|GetAdditionalDamage) 5.0))
      (if (.Value (Utilities|Map|Find (Variables|/Game/Blueprints/BP_VehicularSaveGame.BP_VehicularSaveGame_C|GetUpgradePurchasedStatus (Variables|Default|GetBPVehicularSaveGame)) "DamageUpgrade3"))
        (Variables|Default|SetAdditionalDamage (+ (Variables|Default|GetAdditionalDamage) 1e+01)))
      (CallFunction|SetProjectileSpeedandSpreadMultiplier)
      (else
        (CallFunction|SetProjectileSpeedandSpreadMultiplier)))
    (else
      (CallFunction|SetProjectileSpeedandSpreadMultiplier))))

(event EventBeginPlay
  (bind _asgi_vehicular (Utilities|Casting|CastToGI_Vehicular (Game|GetGameInstance)))
  (bind _output_get (Variables|Default|SetGameInstance _asgi_vehicular))
  (bind _asbp_vehicular_save_game (Utilities|Casting|CastToBP_VehicularSaveGame (Variables|/Script/VehicularGame.VehicularGameInstance|GetSaveGameObject _output_get)))
  (Variables|Default|SetBPVehicularSaveGame _asbp_vehicular_save_game)
  (CallFunction|SetAdditionalMaxHealth))

(event EventTick
  (params (DeltaSeconds :type Float%20%28single-precision%29)))

(fn ConstructionScript)