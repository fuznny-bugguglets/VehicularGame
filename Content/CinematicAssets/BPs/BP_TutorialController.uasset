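; Player-controlled tutorial pawn that lets the player look around and shoot, then loads the Main2 level once three enemies are killed.
; It adds the IM_Cinematic Enhanced Input context on BeginPlay for look and shoot actions.
; Shooting spawns a BP_TutorialProjectile after a short delay at one of two random spawn points, aimed along the actor's forward vector.
; Tick polls EnemiesKilled, which this graph never increments, to trigger the delayed level change.
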(event Custom|check
  (if (== (Variables|Default|GetEnemiesKilled) 3)
    (Utilities|FlowControl|Delay 0.5)
    (Game|OpenLevel(byName) "Main2")))

(event Input|EnhancedActionEvents|EnhancedInputActionIA_CLook
  (params (ActionValue :type Vector%202D%20Structure) (ElapsedSeconds :type Float%20%28double-precision%29) (TriggeredSeconds :type Float%20%28double-precision%29) (InputAction :type Input%20Action%20Object%20Reference :default "/Game/CinematicAssets/Inputs/IA_CLook.IA_CLook"))
  (bind (_x _y) (Math|Vector2D|BreakVector2D ActionValue))
  (Pawn|Input|AddControllerYawInput _x)
  (Pawn|Input|AddControllerPitchInput _y))

(event Input|EnhancedActionEvents|EnhancedInputActionIA_CShoot
  (params (ActionValue :type Boolean) (ElapsedSeconds :type Float%20%28double-precision%29) (TriggeredSeconds :type Float%20%28double-precision%29) (InputAction :type Input%20Action%20Object%20Reference :default "/Game/CinematicAssets/Inputs/IA_CShoot.IA_CShoot"))
  (Utilities|FlowControl|Delay 0.4)
  (Game|SpawnActorfromClass "/Game/CinematicAssets/BPs/BP_TutorialProjectile.BP_TutorialProjectile_C" (Math|Transform|MakeTransform (Transformation|GetWorldLocation (.OutItem (Utilities|Array|Random (Utilities|Array|MakeArray (Variables|Default|GetProjectile%20spawn%20location1) (Variables|Default|GetProjectile%20spawn%20location))))) (Math|Conversions|RotationFromXVector (Transformation|GetActorForwardVector)) "1.000000,1.000000,1.000000") "Undefined" "MultiplyWithRoot" 0 0)
  (Development|PrintString "shot"))

(event EventBeginPlay
  (bind _returnvalue (Game|GetPlayerController 0))
  (bind _returnvalue_2 (PlayerController|LocalPlayerSubsystems|GetEnhancedInputLocalPlayerSubsystem _returnvalue))
  (Utilities|IsValid _returnvalue_2
    (:Is%20Valid
      (Input|AddMappingContext _returnvalue_2 "/Game/CinematicAssets/Inputs/IM_Cinematic.IM_Cinematic" 0 "(bIgnoreAllPressedKeysUntilRelease=True,bForceImmediately=False,bNotifyUserSettings=False)"))))

(event EventTick
  (params (DeltaSeconds :type Float%20%28single-precision%29))
  (CallFunction|Check))

(fn ConstructionScript)